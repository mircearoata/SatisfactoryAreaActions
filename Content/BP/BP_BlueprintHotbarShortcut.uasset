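; BP_BlueprintHotbarShortcut is a hotbar shortcut that starts loading a saved blueprint through the player's Area Actions component.
; On Execute it cancels any current area action on the controlled character, then runs a BP_BlueprintLoad action.
; If that action starts, it receives the shortcut's blueprint file name; otherwise the returned error is logged.
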(event EventExecute
  (params (owner :type FG%20Player%20Controller%20Object%20Reference))
  (bind _returnvalue (Pawn|GetControlledPawn owner))
  (bind _asfgcharacter_player (Utilities|Casting|CastToFGCharacterPlayer _returnvalue))
  (bind _returnvalue_2 (Class|AABlueprintFunctionLibrary|GetAreaActionsComponent _asfgcharacter_player))
  (bind _currentaction (Variables|/Script/AreaActions.AAAreaActionsComponent|GetCurrentAction _returnvalue_2))
  (Utilities|FlowControl|Sequence
    (:then_0
      (if (Utilities|IsValid _currentaction)
        (Class|AAAction|Cancel _currentaction)))
    (:then_1
      (bind (_error _returnvalue_3) (Class|AAAreaActionsComponent|RunAction _returnvalue_2 "/AreaActions/Actions/BlueprintLoad/BP_BlueprintLoad.BP_BlueprintLoad_C"))
      (if _returnvalue_3
        (Default|SetBlueprint (.AsBP%20Blueprint%20Load (Utilities|Casting|CastToBP_BlueprintLoad (Variables|/Script/AreaActions.AAAreaActionsComponent|GetCurrentAction _returnvalue_2))) (Class|AABlueprintHotbarShortcut|GetBlueprintFileName))
        (else
          (Class|BlueprintLoggingLibrary|LogError (Utilities|String|ToString(Text) _error)))))))