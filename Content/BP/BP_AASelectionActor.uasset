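; Area Actions selection actor that shows on-screen key hints while it is in play.
; Shortly after BeginPlay it creates a key hints widget bound to itself, labeling primary fire by the current selection mode (corner, bottom limit, top limit or building).
; Secondary fire is labeled as the actions menu, and build gun toggle or Escape as cancel.
; EndPlay removes the widget.
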(event EventBeginPlay
  (Utilities|FlowControl|Delay 0.01)
  (bind _returnvalue (UserInterface|CreateWidget "/AreaActions/UI/Actions/Widget_KeyHints.Widget_KeyHints_C" 0 (Utilities|Array|MakeArray (Utilities|Struct|MakeStruct_KeybindingHint (Utilities|Select :Index (Class|AASelectionActor|GetSelectionMode) :SM_Corner "Place/Remove Corner" :SM_Bottom "Set/Remove Bottom Limit" :SM_Top "Set/Remove Top Limit" :SM_Building "Add/Remove Building") "{PrimaryFire}") (Utilities|Struct|MakeStruct_KeybindingHint "Area Actions Menu" "{SecondaryFire}") (Utilities|Struct|MakeStruct_KeybindingHint "Cancel" "{ToggleBuildGun} / ESC")) self))
  (bind _output_get (Variables|Default|SetHintsWidget _returnvalue))
  (UserInterface|Viewport|AddtoViewport _output_get 0))

(event EventEndPlay
  (params (EndPlayReason :type EEndPlayReason%20Enum :default "Destroyed"))
  (Widget|RemovefromParent (Variables|Default|GetHintsWidget)))

(fn ConstructionScript)