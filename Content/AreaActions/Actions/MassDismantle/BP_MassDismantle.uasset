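; Mass Dismantle area action that dismantles the selected buildings, wrapped in confirmation prompts shown through the area action equipment.
; Init warns of the building count and a temporary game freeze before asking to proceed.
; PostRun totals the refunded items and asks whether to deliver them in a crate near the player.
; Both prompts pass Yes/No choices to delegates; the dismantle and crate logic are not in these graphs.
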(event EventInit
  (Class|AAEquipment|ShowMessageYesNoDelegate (Variables|Default|GetmAAEquipment) "Mass Dismantle" (Utilities|Text|FormatText "Are you sure you want to dismantle {ActorCount} buildings? 
The game will freeze for a while." (Utilities|Array|Length (Variables|Default|GetmActors))) (EventDispatchers|CreateEvent :!event Run) (EventDispatchers|CreateEvent :!event Done)))

(event EventPostRun
  (for _array_element (Variables|Default|GetmRefunds)
    (Variables|Default|SetTotalRefundItemCount (+ (.out_numItems (Class|FGInventoryLibrary|BreakInventoryStack _array_element)) (Variables|Default|GetTotalRefundItemCount))))
  (Class|AAEquipment|ShowMessageYesNoDelegate (Variables|Default|GetmAAEquipment) "Mass Dismantle" (Utilities|Text|FormatText "Do you want to receive the refunds ({ItemCount} items) in a crate near you?" (Variables|Default|GetTotalRefundItemCount)) (EventDispatchers|CreateEvent :!event GiveRefunds) (EventDispatchers|CreateEvent :!event Done)))

(fn ConstructionScript)