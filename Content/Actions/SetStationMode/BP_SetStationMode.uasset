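; An area action that sets stations to Load or Unload mode.
; Run shows a mode-selection widget, whose result event passes the chosen mode to SetStationMode.
; An OK message then names the changed buildings and their new mode, or reports that the area has no stations.
; Dismissing that message completes the action through Done.
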(event Custom|Result
  (params (IsLoadMode :type Boolean))
  (Variables|Default|SetActionWidget 0)
  (bind _statistics (Class|AASetStationMode|SetStationMode IsLoadMode))
  (if (> (Utilities|Map|Length _statistics) 0)
    (bind _returnvalue (UserInterface|CreateWidget "/AreaActions/UI/Actions/Widget_ActionMessageOk.Widget_ActionMessageOk_C" 0 (Utilities|Text|FormatText "Set {Buildings} to {Mode}" (CallFunction|FormatBuildingNames _statistics) (select IsLoadMode "Load" "Unload"))))
    (EventDispatchers|BindEventtoOnOkClicked _returnvalue (delegate Custom|StatisticsOkClicked))
    (Variables|Default|SetActionWidget _returnvalue)
    (else
      (bind _returnvalue_2 (UserInterface|CreateWidget "/AreaActions/UI/Actions/Widget_ActionMessageOk.Widget_ActionMessageOk_C" 0 "No stations in the area."))
      (EventDispatchers|BindEventtoOnOkClicked _returnvalue_2 (delegate Custom|StatisticsOkClicked))
      (Variables|Default|SetActionWidget _returnvalue_2))))

(event Custom|StatisticsOkClicked
  (Class|AAAction|Done))

(event EventRun
  (bind _returnvalue (UserInterface|CreateWidget "/AreaActions/Actions/SetStationMode/Widget_SetStationMode.Widget_SetStationMode_C"))
  (EventDispatchers|BindEventtoResult _returnvalue (delegate Custom|Result))
  (EventDispatchers|BindEventtoCancel _returnvalue (EventDispatchers|CreateEvent :!event Done))
  (Variables|Default|SetActionWidget _returnvalue))

(fn ConstructionScript)