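; Mass dismantle action that asks the player to confirm before dismantling a batch of buildings and before handing out the resulting refunds.
; Run shows a Yes/No message widget with the building count, and Yes calls Dismantle.
; ShowGiveRefundsWidget totals the refunded item counts into a second prompt, and Yes calls GiveRefunds.
; The Blueprint handles only these prompts, tracked in ActionWidget; the dismantle and refund logic is defined outside this graph.
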(event Custom|Dismantle_Yes
  (Variables|Default|SetActionWidget 0)
  (Class|AAMassDismantle|Dismantle))

(event Custom|GiveRefunds_Yes
  (Variables|Default|SetActionWidget 0)
  (Class|AAMassDismantle|GiveRefunds))

(event EventShowGiveRefundsWidget
  (for _array_element (Variables|Default|GetRefunds)
    (bind _output_get (Variables|Default|SetRefundCount (+ (stale _output_get) (.out_numItems (Class|FGInventoryLibrary|BreakInventoryStack _array_element))))))
  (bind _returnvalue (UserInterface|CreateWidget "/AreaActions/UI/Actions/Widget_ActionMessageYesNo.Widget_ActionMessageYesNo_C" 0 (Utilities|Text|FormatText "Do you want to receive the refunds for {NumItems} items?" _output_get)))
  (EventDispatchers|BindEventtoOnYesClicked _returnvalue (delegate Custom|GiveRefunds_Yes))
  (EventDispatchers|BindEventtoOnNoClicked _returnvalue (EventDispatchers|CreateEvent :!event Done))
  (Variables|Default|SetActionWidget _returnvalue))

(event EventRun
  (bind _returnvalue (UserInterface|CreateWidget "/AreaActions/UI/Actions/Widget_ActionMessageYesNo.Widget_ActionMessageYesNo_C" 0 (Utilities|Text|FormatText "Are you sure you want to dismantle {Num} buildings?" (Utilities|Array|Length (Variables|Default|GetActors)))))
  (EventDispatchers|BindEventtoOnYesClicked _returnvalue (delegate Custom|Dismantle_Yes))
  (EventDispatchers|BindEventtoOnNoClicked _returnvalue (EventDispatchers|CreateEvent :!event Cancel))
  (Variables|Default|SetActionWidget _returnvalue))

(fn ConstructionScript)