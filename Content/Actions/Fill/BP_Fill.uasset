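; BP_Fill is the Fill building action, which starts a placement from the selected actors.
; Run loads the actors into CopyBuildingsComponent, derives the area size from their bounds, enters placing mode, and creates fill, item-cost and key-hint widgets.
; A failed selection shows an OK message, outlining buildings with links outside the selection when no specific error is returned.
; EndPlay removes the cost and hint widgets.
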(event EventRun
  (bind (_outbuildingswithissues _error _returnvalue) (Class|AACopyBuildingsComponent|SetActors (Variables|Default|GetCopyBuildingsComponent) (Variables|Default|GetActors)))
  (if _returnvalue
    (Variables|Default|SetAreaSize (* (Utilities|Struct|BreakAARotatedBoundingBox (Class|AACopyBuildingsComponent|GetBounds (Variables|Default|GetCopyBuildingsComponent))) 2.0))
    (bind _returnvalue_2 (UserInterface|CreateWidget "/AreaActions/Actions/Fill/Widget_Fill.Widget_Fill_C" 0 self))
    (Variables|Default|SetActionWidget _returnvalue_2)
    (Class|AAFill|EnterPlacing)
    (Utilities|FlowControl|Sequence
      (:then_0
        (bind _returnvalue_3 (UserInterface|CreateWidget "/AreaActions/Actions/Fill/Widget_Fill_Building.Widget_Fill_Building_C" 0 "Fill" self))
        (bind _output_get (Variables|Default|SetBuildingWidget _returnvalue_3))
        (bind _returnvalue_4 (Class|AACopyBuildingsComponent|GetRequiredItems (Variables|Default|GetCopyBuildingsComponent)))
        (Default|SetCosts _output_get (CallFunction|MakeItemAmountArray _returnvalue_4))
        (UserInterface|Viewport|AddtoViewport _output_get 0))
      (:then_1
        (bind _returnvalue_5 (UserInterface|CreateWidget "/AreaActions/Actions/Fill/Widget_Fill_KeyHints.Widget_Fill_KeyHints_C" 0 0 0))
        (bind _output_get_2 (Variables|Default|SetHintWidget _returnvalue_5))
        (UserInterface|Viewport|AddtoViewport _output_get_2 0)))
    (elif (Utilities|Text|TextIsEmpty _error)
      (Class|FGOutlineComponent|ShowMultiActorOutline (Actor|GetComponentbyClass (Game|GetPlayerCharacter 0) "/Script/FactoryGame.FGOutlineComponent") _outbuildingswithissues "OC_INVALIDHOLOGRAM")
      (bind _returnvalue_6 (UserInterface|CreateWidget "/AreaActions/UI/Actions/Widget_ActionMessageOk.Widget_ActionMessageOk_C" 0 (Utilities|Text|FormatText "Some buildings have links to other buildings outside the selected area. The buildings with issues are highlighted.")))
      (EventDispatchers|BindEventtoOnOkClicked _returnvalue_6 (EventDispatchers|CreateEvent :!event Done))
      (Variables|Default|SetActionWidget _returnvalue_6)
      (else
        (bind _returnvalue_7 (UserInterface|CreateWidget "/AreaActions/UI/Actions/Widget_ActionMessageOk.Widget_ActionMessageOk_C" 0 _error))
        (EventDispatchers|BindEventtoOnOkClicked _returnvalue_7 (EventDispatchers|CreateEvent :!event Done))
        (Variables|Default|SetActionWidget _returnvalue_7)))))

(event EventEndPlay
  (params (EndPlayReason :type EEndPlayReason%20Enum :default "Destroyed"))
  (Widget|RemovefromParent (Variables|Default|GetBuildingWidget))
  (Widget|RemovefromParent (Variables|Default|GetHintWidget)))

(fn ConstructionScript)

(fn GetInventories
  (return (CallFunction|GetInventories)))