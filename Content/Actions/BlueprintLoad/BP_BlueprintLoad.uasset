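; Action that loads a saved building blueprint from a path and lets it be placed in the world.
; A successful load adds a copy around the buildings' center through BlueprintPlacingComponent, enters placing, and shows load, cost and key hint widgets.
; A failed load shows an OK message widget instead.
; The cost and hint widgets are removed on EndPlay.
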(event Custom|SetBlueprint
  (params (BlueprintPath :type String))
  (bind _blueprintplacingcomponent (Variables|Default|GetBlueprintPlacingComponent))
  (bind _returnvalue (Class|AALoadBlueprint|SetPath BlueprintPath))
  (if _returnvalue
    (Class|AABlueprintPlacingComponent|AddCopy _blueprintplacingcomponent "0, 0, 0" "0, 0, 0" (Class|AABlueprintPlacingComponent|GetBuildingsCenter _blueprintplacingcomponent) true)
    (bind _returnvalue_2 (UserInterface|CreateWidget "/AreaActions/Actions/BlueprintLoad/Widget_BlueprintLoad.Widget_BlueprintLoad_C" 0 self))
    (Variables|Default|SetActionWidget _returnvalue_2)
    (Class|AALoadBlueprint|EnterPlacing)
    (Utilities|FlowControl|Sequence
      (:then_0
        (bind _returnvalue_3 (UserInterface|CreateWidget "/AreaActions/Actions/BlueprintLoad/Widget_BlueprintLoad_Building.Widget_BlueprintLoad_Building_C" 0 "Blueprint" self))
        (bind _output_get (Variables|Default|SetBuildingWidget _returnvalue_3))
        (bind _returnvalue_4 (Class|AABlueprintPlacingComponent|GetRequiredItems (Variables|Default|GetBlueprintPlacingComponent)))
        (Default|SetCosts _output_get (CallFunction|MakeItemAmountArray _returnvalue_4))
        (UserInterface|Viewport|AddtoViewport _output_get 0))
      (:then_1
        (bind _returnvalue_5 (UserInterface|CreateWidget "/AreaActions/Actions/BlueprintLoad/Widget_BlueprintLoad_KeyHints.Widget_BlueprintLoad_KeyHints_C" 0 0 0))
        (bind _output_get_2 (Variables|Default|SetHintWidget _returnvalue_5))
        (UserInterface|Viewport|AddtoViewport _output_get_2 0)))
    (else
      (bind _returnvalue_6 (UserInterface|CreateWidget "/AreaActions/UI/Actions/Widget_ActionMessageOk.Widget_ActionMessageOk_C" 0 (Utilities|Text|FormatText "Blueprint could not be loaded")))
      (EventDispatchers|BindEventtoOnOkClicked _returnvalue_6 (EventDispatchers|CreateEvent :!event Done))
      (Variables|Default|SetActionWidget _returnvalue_6))))

(event EventEndPlay
  (params (EndPlayReason :type EEndPlayReason%20Enum :default "Destroyed"))
  (Widget|RemovefromParent (Variables|Default|GetBuildingWidget))
  (Widget|RemovefromParent (Variables|Default|GetHintWidget)))

(fn ConstructionScript)

(fn GetInventories
  (return (CallFunction|GetInventories)))