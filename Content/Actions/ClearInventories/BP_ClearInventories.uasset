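; BP_ClearInventories is an action that empties the inventories of a set of building actors after the player confirms.
; Run shows a Yes/No widget stating the building count, binding Yes to Confirm_Yes.
; Confirm_Yes calls ClearInventories, then shows an OK widget reporting how many items were cleared.
; Each prompt is handed off through the ActionWidget variable.
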(event Custom|Confirm_Yes
  (Variables|Default|SetActionWidget 0)
  (bind _returnvalue (Class|AAClearInventories|ClearInventories))
  (bind _returnvalue_2 (UserInterface|CreateWidget "/AreaActions/UI/Actions/Widget_ActionMessageOk.Widget_ActionMessageOk_C" 0 (Utilities|Text|FormatText "Cleared {Num} items." _returnvalue)))
  (EventDispatchers|BindEventtoOnOkClicked _returnvalue_2 (EventDispatchers|CreateEvent :!event Done))
  (Variables|Default|SetActionWidget _returnvalue_2))

(event EventRun
  (bind _returnvalue (UserInterface|CreateWidget "/AreaActions/UI/Actions/Widget_ActionMessageYesNo.Widget_ActionMessageYesNo_C" 0 (Utilities|Text|FormatText "Are you sure you want to clear the inventories of {Num} buildings?" (Utilities|Array|Length (Variables|Default|GetActors)))))
  (EventDispatchers|BindEventtoOnYesClicked _returnvalue (delegate Custom|Confirm_Yes))
  (EventDispatchers|BindEventtoOnNoClicked _returnvalue (EventDispatchers|CreateEvent :!event Cancel))
  (Variables|Default|SetActionWidget _returnvalue))

(fn ConstructionScript)