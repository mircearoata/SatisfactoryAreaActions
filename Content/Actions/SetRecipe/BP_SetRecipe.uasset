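; Area action that sets a chosen recipe on the machines that accept it.
; Run shows a recipe selection widget through the action widget slot and the AreaActionsComponent build menu.
; The selected recipe is passed to SetRecipe, and an OK message then reports the changed buildings or that no machines accept it.
; Confirming that message finishes the action.
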(event Custom|RecipeSelected
  (params (Recipe :type FG%20Recipe%20Class%20Reference))
  (Variables|Default|SetActionWidget 0)
  (bind _statistics (Class|AASetRecipe|SetRecipe Recipe))
  (if (> (Utilities|Map|Length _statistics) 0)
    (bind _returnvalue (UserInterface|CreateWidget "/AreaActions/UI/Actions/Widget_ActionMessageOk.Widget_ActionMessageOk_C" 0 (Utilities|Text|FormatText "Set recipe to {Recipe} for {Buildings}" (Class|FGRecipe|GetRecipeName Recipe) (CallFunction|FormatBuildingNames _statistics))))
    (EventDispatchers|BindEventtoOnOkClicked _returnvalue (delegate Custom|StatisticsOkClicked))
    (Variables|Default|SetActionWidget _returnvalue)
    (else
      (bind _returnvalue_2 (UserInterface|CreateWidget "/AreaActions/UI/Actions/Widget_ActionMessageOk.Widget_ActionMessageOk_C" 0 "No machines accept this recipe"))
      (EventDispatchers|BindEventtoOnOkClicked _returnvalue_2 (delegate Custom|StatisticsOkClicked))
      (Variables|Default|SetActionWidget _returnvalue_2))))

(event Custom|StatisticsOkClicked
  (Class|AAAction|Done))

(event EventRun
  (bind _returnvalue (UserInterface|CreateWidget "/AreaActions/Actions/SetRecipe/Widget_SetRecipe.Widget_SetRecipe_C"))
  (EventDispatchers|BindEventtoRecipeSelected _returnvalue (delegate Custom|RecipeSelected))
  (EventDispatchers|BindEventtoCanceled _returnvalue (EventDispatchers|CreateEvent :!event Done))
  (Variables|Default|SetActionWidget _returnvalue)
  (Class|AAAreaActionsComponent|ShowBuildMenu (Variables|Default|GetAreaActionsComponent)))

(fn ConstructionScript)