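; Area action that saves a selection of buildings as a blueprint.
; On run it creates the blueprint object; on success it captures an icon, opens the save widget and shows the build menu through the area actions component.
; On failure it outlines the buildings linked outside the selected area in the invalid-hologram color and shows a message with an OK button.
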(event EventRun
  (bind (_actorswithissues _returnvalue) (Class|AASaveBlueprint|CreateBlueprintObject))
  (if _returnvalue
    (Class|AASaveBlueprint|CaptureIcon)
    (bind _returnvalue_2 (UserInterface|CreateWidget "/AreaActions/Actions/BlueprintSave/Widget_BlueprintSave.Widget_BlueprintSave_C" 0 self))
    (Variables|Default|SetActionWidget _returnvalue_2)
    (Class|AAAreaActionsComponent|ShowBuildMenu (Variables|Default|GetAreaActionsComponent))
    (else
      (Class|FGOutlineComponent|ShowMultiActorOutline (Actor|GetComponentbyClass (Game|GetPlayerCharacter 0) "/Script/FactoryGame.FGOutlineComponent") _actorswithissues "OC_INVALIDHOLOGRAM")
      (bind _returnvalue_3 (UserInterface|CreateWidget "/AreaActions/UI/Actions/Widget_ActionMessageOk.Widget_ActionMessageOk_C" 0 (Utilities|Text|FormatText "Some buildings have links to other buildings outside the selected area. The buildings with issues are highlighted.")))
      (EventDispatchers|BindEventtoOnOkClicked _returnvalue_3 (EventDispatchers|CreateEvent :!event Done))
      (Variables|Default|SetActionWidget _returnvalue_3))))

(fn ConstructionScript)